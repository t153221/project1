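; Player pawn for a top-down game that moves on world axes and rotates to face the mouse cursor.
; Tick projects the cursor ray onto a horizontal plane at the player's height for aim yaw, and pins the audio listener to the player.
; BeginPlay shows the cursor and HUD, and overlapping a BP_Enemy opens the game-over widget.
; Forward-axis input also plays a delayed footstep sound when the player is moving.
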(event EventTick
  (params (DeltaSeconds :type Float%20%28single-precision%29))
  (bind _returnvalue (Transformation|GetActorLocation))
  (bind _returnvalue_2 (Game|GetPlayerController 0))
  (bind (_locationx _locationy) (Game|Player|GetMousePosition _returnvalue_2))
  (bind (_worldlocation _worlddirection) (Class|PlayerController|DeprojectScreenPositiontoWorld _returnvalue_2 _locationx _locationy))
  (Transformation|SetActorRotation (Math|Rotator|MakeRotator 0.0 0.0 (.yaw (Math|Rotator|FindLookatRotation _returnvalue (.Intersection (Class|KismetMathLibrary|LinePlaneIntersectionOriginNormal _worldlocation (+ _worldlocation (* _worlddirection 5e+07)) _returnvalue "0.000000,0.000000,1.000000"))))))
  (Class|PlayerController|SetAudioListenerOverride (Game|GetPlayerController 0) 0 (Transformation|GetActorLocation) "0, 0, 0"))

(event EventBeginPlay
  (Variables|/Script/Engine.PlayerController|SetbShowMouseCursor (Game|GetPlayerController 0) true)
  (bind _returnvalue (UserInterface|CreateWidget "/Game/WBP_HUD.WBP_HUD_C"))
  (UserInterface|Viewport|AddtoViewport _returnvalue 0))

(event Collision|EventActorBeginOverlap
  (params (OtherActor :type Actor%20Object%20Reference))
  (Utilities|Casting|CastToBP_Enemy OtherActor)
  (bind _returnvalue (UserInterface|CreateWidget "/Game/WBP_GameOver.WBP_GameOver_C"))
  (UserInterface|Viewport|AddtoViewport _returnvalue 0))

(event Input|AxisEvents|InputAxisMoveForward
  (params (AxisValue :type Float%20%28single-precision%29))
  (Pawn|Input|AddMovementInput (Math|Vector|MakeVector 1.0 0.0 0.0) AxisValue false)
  (Utilities|FlowControl|Delay 4.5)
  (if (> (Math|Vector|VectorLength (Transformation|GetVelocity)) 1e+01)
    (Audio|PlaySoundatLocation "/Game/521590__fission9__hiking-boot-footsteps-on-stone.521590__fission9__hiking-boot-footsteps-on-stone" (Transformation|GetActorLocation) "0, 0, 0" 1.0 1.0 0.0 0 0 0 0)))

(event Input|AxisEvents|InputAxisMoveRight
  (params (AxisValue :type Float%20%28single-precision%29))
  (Pawn|Input|AddMovementInput (Math|Vector|MakeVector 0.0 1.0 0.0) AxisValue false))

(event Input|AxisEvents|InputAxisMoveBack
  (params (AxisValue :type Float%20%28single-precision%29))
  (Pawn|Input|AddMovementInput (Math|Vector|MakeVector -1.0 0.0 0.0) AxisValue false))

(event Input|AxisEvents|InputAxisMoveLeft
  (params (AxisValue :type Float%20%28single-precision%29))
  (Pawn|Input|AddMovementInput (Math|Vector|MakeVector 0.0 -1.0 0.0) AxisValue false))

(fn ConstructionScript)